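; Base player weapon actor that displays a 2D flipbook weapon and animates its draw and bob motion.
; A SceneCaptureComponent2D captures only the weapon flipbook, which InitializeWeapon sets and hides in game.
; DrawWeapon and BobGun use timelines to lerp the flipbook's relative location between draw, rest and bob positions.
; When bobbing is disallowed, BobGun eases the flipbook from its current location back to rest.
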(event Custom|BobGun
  (params (CanBob :type Boolean))
  (bind _newtrack_0 (Timeline|HeadBob Play)
    (:Update
      (if CanBob
        (Transformation|SetRelativeLocation (Variables|Default|GetWeaponFlipBook) (Math|Vector|Lerp(Vector) (Variables|Default|GetWeaponPosition) (Variables|Default|GetWeaponBobPosition) _newtrack_0) false false)
        (else
          (Transformation|SetRelativeLocation (Variables|Default|GetWeaponFlipBook) (Math|Vector|Lerp(Vector) (Variables|/Script/Engine.SceneComponent|GetRelativeLocation (Variables|Default|GetWeaponFlipBook)) (Variables|Default|GetWeaponPosition) _newtrack_0) false false))))))

(event Custom|DrawWeapon
  (bind _newtrack_0 (Timeline|Draw Play)
    (:Update
      (Transformation|SetRelativeLocation (Variables|Default|GetWeaponFlipBook) (Math|Vector|Lerp(Vector) (Variables|Default|GetWeaponDrawPosition) (Variables|Default|GetWeaponPosition) _newtrack_0) false false))))

(event EventBeginPlay
  (Rendering|SceneCapture|ShowOnlyComponent (Variables|Default|GetSceneCaptureComponent2D) (Variables|Default|GetWeaponFlipBook)))

(event Collision|EventActorBeginOverlap
  (params (OtherActor :type Actor%20Object%20Reference)))

(event EventTick
  (params (DeltaSeconds :type Float%20%28single-precision%29)))

(event EventInitializeWeapon
  (bind _weaponflipbook (Variables|Default|GetWeaponFlipBook))
  (Sprite|SetFlipbook _weaponflipbook)
  (Development|SetHiddeninGame _weaponflipbook true false))

(fn ConstructionScript)