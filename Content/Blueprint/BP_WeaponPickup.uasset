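; BP_WeaponPickup is a weapon pickup actor that equips the player with a configured weapon on touch.
; When a BP_player overlaps it, it passes WeaponToPickup to the player's EquipWeapon and then destroys itself.
; Every tick it yaws the WeaponPickup component toward the player camera with a 90-degree offset, billboard-style, keeping pitch and roll at zero.
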(event EventBeginPlay)

(event Collision|EventActorBeginOverlap
  (params (OtherActor :type Actor%20Object%20Reference))
  (bind _asbp_player (Utilities|Casting|CastToBP_player OtherActor))
  (Default|EquipWeapon _asbp_player (Variables|WeaponPickup|GetWeapon%20to%20pickup))
  (Actor|DestroyActor))

(event EventTick
  (params (DeltaSeconds :type Float%20%28single-precision%29))
  (bind _weapon_pickup (Variables|Default|GetWeapon%20Pickup))
  (Transformation|SetWorldRotation _weapon_pickup (Math|Rotator|MakeRotator 0.0 0.0 (- (.yaw (Math|Rotator|FindLookatRotation (Transformation|GetWorldLocation _weapon_pickup) (Camera|GetCameraLocation (Game|GetPlayerCameraManager 0)))) 9e+01)) false false))

(fn ConstructionScript)